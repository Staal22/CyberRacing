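; BP_Arrow_spline is a construction-time placement tool that repeats a chosen mesh, presumably arrow props, along an editable spline.
; The construction script derives spacing from the mesh's X bounding-box size plus Offset, then fills the spline length with Hierarchical Instanced Static Mesh instances.
; Each unit-scale instance sits at a local-space distance along the spline, its X axis aimed at the next point.
; The event graph has no active logic.
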(fn `GetlocationAtIndex`
  (params (A :type Integer))
  (returns (ReturnValue :type "Vector Structure"))
  (return (`SplineComponent.GetLocationAtDistanceAlongSpline` (`self.Spline`) (* A (`self.spacing`)) "Local")))

(fn `UserConstructionScript`
  (locals (NewLocalVar_0 :type Integer :default 0))
  (bind (_min _max) (break `Box` (`StaticMesh.GetBoundingBox` (`self.Place Mesh`))))
  (`StaticMeshComponent.SetStaticMesh` (`self.HierarchicalInstancedStaticMesh`) (`self.Place Mesh`))
  (bind _output_get (set `self.spacing` (+ (.x (- _max _min)) (`self.offset`))))
  (bind _output_get_2 (set `local.NewLocalVar_0` (`KismetMathLibrary.FFloor` (/ (`SplineComponent.GetSplineLength` (`self.Spline`)) _output_get))))
  (for _index (range (+ _output_get_2 1))
    (bind _returnvalue (`self.GetlocationAtIndex` _index))
    (`InstancedStaticMeshComponent.AddInstance` (`self.HierarchicalInstancedStaticMesh`) (`KismetMathLibrary.MakeTransform` _returnvalue (`KismetMathLibrary.MakeRotFromX` (- (`self.GetlocationAtIndex` (+ _index 1)) _returnvalue))))))