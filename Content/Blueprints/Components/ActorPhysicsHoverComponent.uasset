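; Hover component that enables physics on its owner's first primitive component and floats it above surfaces using forces applied each tick.
; A downward GravityTrace scales Gravity by distance along the hit normal; without a hit, full Gravity acts along the component's up vector.
; Within that hit branch, a TraceLength trace adds an eased HoverForce that weakens with distance, plus linear and angular damping.
; Both traces point world-down on the Visibility channel.
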(event `self.ReceiveBeginPlay`
  (`PrimitiveComponent.SetSimulatePhysics` (`Actor.GetComponentByClass` (`self.GetOwner`) "/Script/Engine.PrimitiveComponent") true))

(event `self.ReceiveTick`
  (params (DeltaSeconds :type "Float (single-precision)"))
  (bind _returnvalue (`Actor.GetComponentByClass` (`self.GetOwner`) "/Script/Engine.PrimitiveComponent"))
  (bind _returnvalue_2 (`self.K2_GetComponentLocation` _returnvalue))
  (bind _returnvalue_3 (`self.K2_GetComponentLocation` _returnvalue))
  (bind (_outhit _returnvalue_4) (`KismetSystemLibrary.LineTraceSingle` _returnvalue_3 (- _returnvalue_3 (`KismetMathLibrary.MakeVector` 0.0 0.0 (`self.GravityTrace`))) "TraceTypeQuery1"))
  (if _returnvalue_4
    (bind (_bblockinghit _binitialoverlap _time _distance _location _impactpoint _normal _impactnormal) (`GameplayStatics.BreakHitResult` _outhit))
    (bind _returnvalue_5 (`KismetMathLibrary.VSize` (- _location (`self.K2_GetComponentLocation`))))
    (if (> _returnvalue_5 0.0)
      (`PrimitiveComponent.AddForce` _returnvalue (* _impactnormal (`KismetMathLibrary.Lerp` 0.0 (`self.Gravity`) (`KismetMathLibrary.Abs` (- (/ _returnvalue_5 (`self.TraceLength`)) 1.0)))) "None" false)
      (bind (_outhit_2 _returnvalue_6) (`KismetSystemLibrary.LineTraceSingle` _returnvalue_2 (- _returnvalue_2 (`KismetMathLibrary.MakeVector` 0.0 0.0 (`self.TraceLength`))) "TraceTypeQuery1"))
      (if _returnvalue_6
        (bind (_bblockinghit_2 _binitialoverlap_2 _time_2 _distance_2 _location_2 _impactpoint_2 _normal_2 _impactnormal_2) (`GameplayStatics.BreakHitResult` _outhit_2))
        (`PrimitiveComponent.AddForce` _returnvalue (* _impactnormal_2 (`KismetMathLibrary.FInterpEaseInOut` (`self.HoverForce`) 0.0 (/ (`KismetMathLibrary.VSize` (- _location_2 (`self.K2_GetComponentLocation`))) (`self.TraceLength`)) 1.0)) "None" false)
        (`PrimitiveComponent.SetLinearDamping` _returnvalue (`self.LinearDamping`))
        (`PrimitiveComponent.SetAngularDamping` _returnvalue (`self.AngularDamping`))))
    (else
      (`PrimitiveComponent.AddForce` _returnvalue (* (`self.GetUpVector`) (`self.Gravity`)) "None" false))))