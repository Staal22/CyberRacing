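; Actor component that caches its owner's SplineComponent on BeginPlay and offers a Mirror function to reshape that spline.
; Mirror replaces each point's location with the spline's right vector there scaled by a fixed negative distance, then updates the spline once.
; It looks up that vector by passing local point locations as world locations.
; A true plane reflection of locations, tangents and up vectors via MirrorVectorByNormal exists only as disconnected, never-run logic.
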(event `self.ReceiveBeginPlay`
  ;[1 1 1] Get spline reference
  (set `self.SplineToMirror` (`Actor.GetComponentByClass` (`self.GetOwner`) "/Script/Engine.SplineComponent")))

(fn `Mirror`
  (bind _splinetomirror (`self.SplineToMirror`))
  (for _index (range (`SplineComponent.GetNumberOfSplinePoints` _splinetomirror))
    (`SplineComponent.SetLocationAtSplinePoint` _splinetomirror _index (* (`SplineComponent.FindRightVectorClosestToWorldLocation` _splinetomirror (`SplineComponent.GetLocationAtSplinePoint` _splinetomirror _index "Local") "Local") -1250.0) "Local" false))
  (`SplineComponent.UpdateSpline` _splinetomirror))