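; Scene component that makes its owner's physics-simulated static mesh hover above surfaces.
; BeginPlay enables physics on the mesh, then each tick a visibility line trace runs straight down from the component.
; On a hit, it pushes the mesh along the surface normal, with force fading linearly to zero at full trace length.
; Linear and angular damping are also set on hits and never reset afterwards.
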(event `self.ReceiveBeginPlay`
  (`PrimitiveComponent.SetSimulatePhysics` (`Actor.GetComponentByClass` (`self.GetOwner`) "/Script/Engine.StaticMeshComponent") true))

(event `self.ReceiveTick`
  (params (DeltaSeconds :type "Float (single-precision)"))
  (bind _returnvalue (`self.K2_GetComponentLocation`))
  (bind _returnvalue_2 (`Actor.GetComponentByClass` (`self.GetOwner`) "/Script/Engine.StaticMeshComponent"))
  (bind (_outhit _returnvalue_3) (`KismetSystemLibrary.LineTraceSingle` _returnvalue (- _returnvalue (`KismetMathLibrary.MakeVector` 0.0 0.0 (`self.TraceLength`))) "TraceTypeQuery1"))
  (if _returnvalue_3
    (bind (_bblockinghit _binitialoverlap _time _distance _location _impactpoint _normal _impactnormal) (`GameplayStatics.BreakHitResult` _outhit))
    (`PrimitiveComponent.AddForce` _returnvalue_2 (* _impactnormal (`KismetMathLibrary.Lerp` (`self.HoverForce`) 0.0 (/ (`KismetMathLibrary.VSize` (- _location (`self.K2_GetComponentLocation`))) (`self.TraceLength`)))) "None" false)
    (`PrimitiveComponent.SetLinearDamping` _returnvalue_2 (`self.LinearDamping`))
    (`PrimitiveComponent.SetAngularDamping` _returnvalue_2 (`self.AngularDamping`))))