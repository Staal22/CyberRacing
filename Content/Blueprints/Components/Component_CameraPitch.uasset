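; Actor component that automatically adjusts the pitch of its owner's camera according to what lies ahead of it.
; Each tick it line-traces along the camera's forward vector for a set length.
; A hit pitches the camera up and a miss pitches it down, while hits on the Invisible physical material leave it unchanged.
; Rotation interpolates toward a one-degree offset from the current pitch, preserving roll and yaw.
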(event `self.ReceiveTick`
  (params (DeltaSeconds :type "Float (single-precision)"))
  (bind _returnvalue (`GameplayStatics.GetWorldDeltaSeconds`))
  (bind _returnvalue_2 (`Actor.GetComponentByClass` (`self.GetOwner`) "/Script/Engine.CameraComponent"))
  (bind _returnvalue_3 (`self.K2_GetComponentRotation` _returnvalue_2))
  (bind _returnvalue_4 (`self.K2_GetComponentLocation` _returnvalue_2))
  (bind (_outhit _returnvalue_5) (`KismetSystemLibrary.LineTraceSingle` _returnvalue_4 (+ _returnvalue_4 (* (`KismetMathLibrary.Normal` (`KismetMathLibrary.GetForwardVector` (`self.K2_GetComponentRotation` _returnvalue_2))) (`self.TraceLength`))) "TraceTypeQuery4" true))
  (if _returnvalue_5
    (if (!= (`.PhysMat` (`GameplayStatics.BreakHitResult` _outhit)) "/Game/Materials/PhysicsMaterials/Invisible.Invisible")
      (`self.K2_SetWorldRotation` _returnvalue_2 (`KismetMathLibrary.RInterpTo` _returnvalue_3 (`KismetMathLibrary.MakeRotator` (.roll _returnvalue_3) (+ (.pitch _returnvalue_3) 1.0) (.yaw _returnvalue_3)) _returnvalue (`self.InterpolationSpeed`)) false false))
    (else
      (`self.K2_SetWorldRotation` _returnvalue_2 (`KismetMathLibrary.RInterpTo` _returnvalue_3 (`KismetMathLibrary.MakeRotator` (.roll _returnvalue_3) (- (.pitch _returnvalue_3) 1.0) (.yaw _returnvalue_3)) _returnvalue (`self.InterpolationSpeed`)) false false))))