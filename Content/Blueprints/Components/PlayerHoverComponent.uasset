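; Hover component for the player car that enables physics on its owner and applies suspension-like forces every tick.
; Traces along the car mesh's down axis drive a distance-scaled Gravity force beyond TraceLength and an eased hover force, plus damping, on short-trace hits.
; Without a surface hit it applies Gravity along its up vector; during a roll it applies no force.
; Both mesh-axis trace endpoints omit the start location offset.
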(event `self.ReceiveBeginPlay`
  (`PrimitiveComponent.SetSimulatePhysics` (`Actor.GetComponentByClass` (`self.GetOwner`) "/Script/Engine.PrimitiveComponent") true))

(event `self.ReceiveTick`
  (params (DeltaSeconds :type "Float (single-precision)"))
  (bind _returnvalue (`self.K2_GetComponentLocation`))
  (bind _gravitytrace (`self.GravityTrace`))
  (bind _returnvalue_2 (`Actor.GetComponentByClass` (`self.GetOwner`) "/Script/Engine.PrimitiveComponent"))
  (bind _asbp_player_car (cast `/Game/Blueprints/Actors/BP_PlayerCar` (`GameplayStatics.GetPlayerPawn` 0)))
  (if (`PlayerCar.bDoARoll` _asbp_player_car)
    (`KismetSystemLibrary.LineTraceSingle` _returnvalue (- _returnvalue (`KismetMathLibrary.MakeVector` 0.0 0.0 _gravitytrace)) "TraceTypeQuery1")
    (else
      (bind (_outhit _returnvalue_3) (`KismetSystemLibrary.LineTraceSingle` _returnvalue (* (`KismetMathLibrary.GetUpVector` (`self.K2_GetComponentRotation` (`PlayerCar.PlayerMesh` _asbp_player_car))) (* _gravitytrace -1.0)) "TraceTypeQuery1"))
      (if _returnvalue_3
        (bind _asbp_player_car_2 (cast `/Game/Blueprints/Actors/BP_PlayerCar` (`GameplayStatics.GetPlayerPawn` 0)))
        (bind (_bblockinghit _binitialoverlap _time _distance _location _impactpoint _normal _impactnormal) (`GameplayStatics.BreakHitResult` _outhit))
        (bind _returnvalue_4 (`KismetMathLibrary.VSize` (- _location (`self.K2_GetComponentLocation`))))
        (bind _tracelength (`PlayerCar.TraceLength` _asbp_player_car_2))
        (if (> _returnvalue_4 _tracelength)
          (`PrimitiveComponent.AddForce` _returnvalue_2 (* _impactnormal (`KismetMathLibrary.Lerp` 0.0 (`self.Gravity`) (`KismetMathLibrary.Abs` (- (/ _returnvalue_4 _tracelength) 1.0)))) "None" false))
        (bind _asbp_player_car_3 (cast `/Game/Blueprints/Actors/BP_PlayerCar` (`GameplayStatics.GetPlayerPawn` 0)))
        (bind (_outhit_2 _returnvalue_5) (`KismetSystemLibrary.LineTraceSingle` (`self.K2_GetComponentLocation`) (* (* (`KismetMathLibrary.GetUpVector` (`self.K2_GetComponentRotation` (`PlayerCar.PlayerMesh` _asbp_player_car_3))) -1.0) (`PlayerCar.TraceLength` _asbp_player_car_3)) "TraceTypeQuery1"))
        (if _returnvalue_5
          (bind _asbp_player_car_4 (cast `/Game/Blueprints/Actors/BP_PlayerCar` (`GameplayStatics.GetPlayerPawn` 0)))
          (bind _asbp_player_car_5 (cast `/Game/Blueprints/Actors/BP_PlayerCar` (`GameplayStatics.GetPlayerPawn` 0)))
          (bind (_bblockinghit_2 _binitialoverlap_2 _time_2 _distance_2 _location_2 _impactpoint_2 _normal_2 _impactnormal_2) (`GameplayStatics.BreakHitResult` _outhit_2))
          (`PrimitiveComponent.AddForce` _returnvalue_2 (* _impactnormal_2 (`KismetMathLibrary.FInterpEaseInOut` (`PlayerCar.HoverForce` _asbp_player_car_5) 0.0 (/ (`KismetMathLibrary.VSize` (- _location_2 (`self.K2_GetComponentLocation`))) (`PlayerCar.TraceLength` _asbp_player_car_4)) 1.0)) "None" false)
          (`PrimitiveComponent.SetLinearDamping` _returnvalue_2 (`self.LinearDamping`))
          (`PrimitiveComponent.SetAngularDamping` _returnvalue_2 (`self.AngularDamping`)))
        (else
          (bind _asbp_player_car_6 (cast `/Game/Blueprints/Actors/BP_PlayerCar` (`GameplayStatics.GetPlayerPawn` 0)))
          (if (not (`PlayerCar.bDoARoll` _asbp_player_car_6))
            (`PrimitiveComponent.AddForce` _returnvalue_2 (* (`self.GetUpVector`) (`self.Gravity`)) "None" false)))))))