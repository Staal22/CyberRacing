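; Actor component that hovers its owner above surfaces below by vertically offsetting the owner's primitive component.
; Each tick it line-traces downward on Visibility from that component over TraceLength.
; On a hit, it interpolates from the component's absolute world Z toward the HoverHeight error, using InterpolationSpeed.
; The interpolated result is applied directly as an unswept world-offset delta, rather than as a position.
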(event `self.ReceiveBeginPlay`)

(event `self.ReceiveTick`
  (params (DeltaSeconds :type "Float (single-precision)"))
  (bind _returnvalue (`Actor.GetComponentByClass` (`self.GetOwner`) "/Script/Engine.PrimitiveComponent"))
  (bind _returnvalue_2 (`self.K2_GetComponentLocation` _returnvalue))
  (bind _returnvalue_3 (`self.K2_GetComponentLocation` _returnvalue))
  (bind (_outhit _returnvalue_4) (`KismetSystemLibrary.LineTraceSingle` _returnvalue_3 (- _returnvalue_3 (`KismetMathLibrary.MakeVector` 0.0 0.0 (`self.TraceLength`))) "TraceTypeQuery1"))
  (if _returnvalue_4
    (`self.K2_AddWorldOffset` _returnvalue (`KismetMathLibrary.VInterpTo` (`KismetMathLibrary.MakeVector` 0.0 0.0 (.z _returnvalue_2)) (`KismetMathLibrary.MakeVector` 0.0 0.0 (- (`self.HoverHeight`) (- (.z _returnvalue_2) (.z (`.Location` (`GameplayStatics.BreakHitResult` _outhit)))))) (`GameplayStatics.GetWorldDeltaSeconds`) (`self.InterpolationSpeed`)) false false)))