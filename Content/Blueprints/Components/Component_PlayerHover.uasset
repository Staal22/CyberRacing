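; Player hover component that simulates a hovercar suspension through physics forces on its owner, using downward traces every tick.
; Beyond hover height, GravityForce acts along the ground normal, scaled by distance; a shorter trace applies eased HoverForce and sets damping.
; With no ground or during HitState, GravityForce follows the component's up vector unless DoARoll is set.
; Tuning and state flags come from BP_PlayerCar, repeatedly cast from player pawn 0.
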(event `self.ReceiveBeginPlay`
  ;[1 1 1] Get Root
  (`PrimitiveComponent.SetSimulatePhysics` (`Actor.GetComponentByClass` (`self.GetOwner`) "/Script/Engine.PrimitiveComponent") true))

(event `self.ReceiveTick`
  (params (DeltaSeconds :type "Float (single-precision)"))
  (bind _returnvalue (`self.K2_GetComponentLocation`))
  (bind _returnvalue_2 (`self.K2_GetComponentLocation`))
  (bind _returnvalue_3 (`Actor.GetComponentByClass` (`self.GetOwner`) "/Script/Engine.PrimitiveComponent"))
  (bind (_outhit _returnvalue_4) (`KismetSystemLibrary.LineTraceSingle` _returnvalue_2 (- _returnvalue_2 (`KismetMathLibrary.MakeVector` 0.0 0.0 (`self.GravityTrace`))) "TraceTypeQuery1"))
  (if _returnvalue_4
    (bind _asbp_player_car (cast `/Game/Blueprints/Actors/BP_PlayerCar` (`GameplayStatics.GetPlayerPawn` 0)))
    (if (`PlayerCar.bHitState` _asbp_player_car)
      (bind _asbp_player_car_2 (cast `/Game/Blueprints/Actors/BP_PlayerCar` (`GameplayStatics.GetPlayerPawn` 0) :!label _label))
      (bind _asbp_player_car_3 (cast `/Game/Blueprints/Actors/BP_PlayerCar` (`GameplayStatics.GetPlayerPawn` 0)))
      (if (not (`PlayerCar.bDoARoll` _asbp_player_car_3))
        (`PrimitiveComponent.AddForce` _returnvalue_3 (* (`self.GetUpVector`) (`PlayerCar.GravityForce` _asbp_player_car_2)) "None" false))
      (else
        (bind _asbp_player_car_4 (cast `/Game/Blueprints/Actors/BP_PlayerCar` (`GameplayStatics.GetPlayerPawn` 0)))
        (bind (_bblockinghit _binitialoverlap _time _distance _location _impactpoint _normal _impactnormal) (`GameplayStatics.BreakHitResult` _outhit))
        (bind _returnvalue_5 (`KismetMathLibrary.VSize` (- _location (`self.K2_GetComponentLocation`))))
        (bind _tracelength (`PlayerCar.TraceLength` _asbp_player_car_4))
        (if (> _returnvalue_5 _tracelength)
          (bind _asbp_player_car_5 (cast `/Game/Blueprints/Actors/BP_PlayerCar` (`GameplayStatics.GetPlayerPawn` 0)))
          (`PrimitiveComponent.AddForce` _returnvalue_3 (* _impactnormal (`KismetMathLibrary.Lerp` 0.0 (`PlayerCar.GravityForce` _asbp_player_car_5) (`KismetMathLibrary.Abs` (- (/ _returnvalue_5 _tracelength) 1.0)))) "None" false))
        (bind _asbp_player_car_6 (cast `/Game/Blueprints/Actors/BP_PlayerCar` (`GameplayStatics.GetPlayerPawn` 0)))
        (bind (_outhit_2 _returnvalue_6) (`KismetSystemLibrary.LineTraceSingle` _returnvalue (- _returnvalue (`KismetMathLibrary.MakeVector` 0.0 0.0 (`PlayerCar.TraceLength` _asbp_player_car_6))) "TraceTypeQuery1"))
        (if _returnvalue_6
          (bind _asbp_player_car_7 (cast `/Game/Blueprints/Actors/BP_PlayerCar` (`GameplayStatics.GetPlayerPawn` 0)))
          (bind _asbp_player_car_8 (cast `/Game/Blueprints/Actors/BP_PlayerCar` (`GameplayStatics.GetPlayerPawn` 0)))
          (if (not (`PlayerCar.bHitState` _asbp_player_car_8))
            (bind (_bblockinghit_2 _binitialoverlap_2 _time_2 _distance_2 _location_2 _impactpoint_2 _normal_2 _impactnormal_2) (`GameplayStatics.BreakHitResult` _outhit_2))
            (`PrimitiveComponent.AddForce` _returnvalue_3 (* _impactnormal_2 (`KismetMathLibrary.FInterpEaseInOut` (`PlayerCar.HoverForce` _asbp_player_car_8) 0.0 (/ (`KismetMathLibrary.VSize` (- _location_2 (`self.K2_GetComponentLocation`))) (`PlayerCar.TraceLength` _asbp_player_car_7)) 2.0)) "None" false)
            (`PrimitiveComponent.SetLinearDamping` _returnvalue_3 (`self.LinearDamping`))
            (`PrimitiveComponent.SetAngularDamping` _returnvalue_3 (`self.AngularDamping`))))))
    (else
      (goto _label))))