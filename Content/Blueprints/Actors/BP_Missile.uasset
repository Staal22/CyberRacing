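; Missile actor that follows the track surface and turns to home in on enemies.
; Each tick, a downward trace gates steering: with WallFollow on, a side trace finds the wall and RInterpTo aligns the mesh's pitch to the ground and yaw to the wall.
; An enemy entering EnemyTrack switches wall following off and tracking on, snapping the actor to face overlapping BP_Enemy or BP_EnemyC_WithNavComponent actors.
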(event `self.ReceiveTick`
  (params (DeltaSeconds :type "Float (single-precision)"))
  (bind _returnvalue (`self.K2_GetActorLocation`))
  (bind _bulletmesh (`self.BulletMesh`))
  (bind _bulletmesh_2 (`self.BulletMesh`))
  (bind _returnvalue_2 (`SceneComponent.K2_GetComponentLocation` _bulletmesh_2))
  (bind _returnvalue_3 (`SceneComponent.K2_GetComponentRotation` _bulletmesh))
  (bind _returnvalue_4 (`SceneComponent.K2_GetComponentLocation` (`self.BulletMesh`)))
  ;[1 1 1] Hovering
  (bind (_outhit _returnvalue_5) (`KismetSystemLibrary.LineTraceSingle` _returnvalue_4 (- _returnvalue_4 (`KismetMathLibrary.MakeVector` 0.0 0.0 (`self.TraceLengthZ`))) "TraceTypeQuery1"))
  (if _returnvalue_5
    ;[1 1 1] Track Enemy
    (if (`self.ToTrack`)
      (for _array_element (`PrimitiveComponent.GetOverlappingActors` (`self.EnemyTrack`) null)
        (bind _asbp_enemy (cast `/Game/Blueprints/Actors/BP_Enemy` _array_element)
          (:`then`
            (`self.K2_SetActorRotation` (`KismetMathLibrary.FindLookAtRotation` _returnvalue (`self.K2_GetActorLocation` _asbp_enemy))))
          (:`CastFailed`
            (bind _asbp_enemy_c_with_nav_component (cast `/Game/Blueprints/Actors/BP_EnemyC_WithNavComponent` _array_element))
            (`self.K2_SetActorRotation` (`KismetMathLibrary.FindLookAtRotation` _returnvalue (`self.K2_GetActorLocation` _asbp_enemy_c_with_nav_component))))))
      (else
        ;[1 1 1] Attempt to follow track
        (if (`self.WallFollow`)
          (bind (_outhit_2 _returnvalue_6) (`KismetSystemLibrary.LineTraceSingle` _returnvalue_2 (- _returnvalue_2 (* (`SceneComponent.GetRightVector` _bulletmesh_2) (`self.TraceLengthY`))) "TraceTypeQuery1" false (`|MakeArray` (`GameplayStatics.GetPlayerPawn` 0) :!type "Actor Object Reference")))
          (if _returnvalue_6
            (`SceneComponent.K2_SetWorldRotation` (`self.BulletMesh`) (`KismetMathLibrary.RInterpTo` _returnvalue_3 (`KismetMathLibrary.MakeRotator` (.roll _returnvalue_3) (.pitch (`KismetMathLibrary.MakeRotFromYZ` (`SceneComponent.GetRightVector` _bulletmesh) (`.ImpactNormal` (`GameplayStatics.BreakHitResult` _outhit)))) (.yaw (`KismetMathLibrary.MakeRotFromZY` (`SceneComponent.GetUpVector` _bulletmesh) (`.ImpactNormal` (`GameplayStatics.BreakHitResult` _outhit_2))))) (`GameplayStatics.GetWorldDeltaSeconds`)) false false)))))))

(event `self.ReceiveBeginPlay`
  ;[1 1 1] Enemy Overlap Check
  (add `PrimitiveComponent.OnComponentBeginOverlap` (`self.EnemyTrack`) (delegate `OnComponentBeginOverlap_Event_0`)))

(event `OnComponentBeginOverlap_Event_0`
  (params (OverlappedComponent :type "PrimitiveComponent Object Reference") (OtherActor :type "Actor Object Reference") (OtherComp :type "PrimitiveComponent Object Reference") (OtherBodyIndex :type Integer) (bFromSweep :type Boolean) (SweepResult :type "HitResult Structure (by ref)"))
  (bind _returnvalue (`self.K2_GetActorLocation`))
  ;[1 1 1] Enemy Overlap Check
  (bind _asbp_enemy (cast `/Game/Blueprints/Actors/BP_Enemy` OtherActor)
    (:`then`
      (`self.K2_SetActorRotation` (`KismetMathLibrary.FindLookAtRotation` _returnvalue (`self.K2_GetActorLocation` _asbp_enemy))))
    (:`CastFailed`
      (bind _asbp_enemy_c_with_nav_component (cast `/Game/Blueprints/Actors/BP_EnemyC_WithNavComponent` OtherActor))
      (`self.K2_SetActorRotation` (`KismetMathLibrary.FindLookAtRotation` _returnvalue (`self.K2_GetActorLocation` _asbp_enemy_c_with_nav_component)))))
  (set `self.WallFollow` false)
  (set `self.ToTrack` true))

(event `self.ReceiveDestroyed`
  ;[1 1 1] On Destroyed
  (set `self.ToTrack` false))

(fn `UserConstructionScript`)