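; Missile projectile that follows the track, homes in on AI cars and calls Missile() on any it hits.
; Each tick, while a downward trace hits, it eases mesh pitch to the ground normal and yaw to a side-wall normal.
; Wall following and hit detection start after a short launch delay.
; An AI car entering EnemyTrack switches it to look-at homing; player-car targeting nodes are left unwired.
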(event `OnComponentBeginOverlap_Event_1`
  (params (OverlappedComponent :type "PrimitiveComponent Object Reference") (OtherActor :type "Actor Object Reference") (OtherComp :type "PrimitiveComponent Object Reference") (OtherBodyIndex :type Integer) (bFromSweep :type Boolean) (SweepResult :type "HitResult Structure (by ref)"))
  (bind _asbp_aicar (cast `/Game/Blueprints/Actors/BP_AICar` OtherActor))
  (`AICar.Missile` _asbp_aicar))

(event `self.ReceiveTick`
  (params (DeltaSeconds :type "Float (single-precision)"))
  (bind _bulletmesh (`self.BulletMesh`))
  (bind _bulletmesh_2 (`self.BulletMesh`))
  (bind _returnvalue (`SceneComponent.K2_GetComponentLocation` _bulletmesh_2))
  (bind _returnvalue_2 (`SceneComponent.K2_GetComponentRotation` _bulletmesh))
  (bind _returnvalue_3 (`SceneComponent.K2_GetComponentLocation` (`self.BulletMesh`)))
  ;[1 1 1] Hovering
  (bind (_outhit _returnvalue_4) (`KismetSystemLibrary.LineTraceSingle` _returnvalue_3 (- _returnvalue_3 (`KismetMathLibrary.MakeVector` 0.0 0.0 (`self.TraceLengthZ`))) "TraceTypeQuery1"))
  (if _returnvalue_4
    ;[1 1 1] Track Enemy
    (if (`self.ToTrack`)
      (for _array_element (`PrimitiveComponent.GetOverlappingActors` (`self.EnemyTrack`) null)
        (bind _asbp_aicar (cast `/Game/Blueprints/Actors/BP_AICar` _array_element))
        (`self.K2_SetActorRotation` (`KismetMathLibrary.FindLookAtRotation` (`self.K2_GetActorLocation`) (`self.K2_GetActorLocation` _asbp_aicar))))
      (else
        ;[1 1 1] Attempt to follow track
        (if (`self.WallFollow`)
          (bind (_outhit_2 _returnvalue_5) (`KismetSystemLibrary.LineTraceSingle` _returnvalue (- _returnvalue (* (`SceneComponent.GetRightVector` _bulletmesh_2) (`self.TraceLengthY`))) "TraceTypeQuery1" false (`|MakeArray` (`GameplayStatics.GetPlayerPawn` 0) :!type "Actor Object Reference")))
          (if _returnvalue_5
            (`SceneComponent.K2_SetWorldRotation` (`self.BulletMesh`) (`KismetMathLibrary.RInterpTo` _returnvalue_2 (`KismetMathLibrary.MakeRotator` (.roll _returnvalue_2) (.pitch (`KismetMathLibrary.MakeRotFromYZ` (`SceneComponent.GetRightVector` _bulletmesh) (`.ImpactNormal` (`GameplayStatics.BreakHitResult` _outhit)))) (.yaw (`KismetMathLibrary.MakeRotFromZY` (`SceneComponent.GetUpVector` _bulletmesh) (`.ImpactNormal` (`GameplayStatics.BreakHitResult` _outhit_2))))) (`GameplayStatics.GetWorldDeltaSeconds`)) false false)))))))

(event `self.ReceiveBeginPlay`
  ;[1 1 1] Enemy Overlap Check
  (add `PrimitiveComponent.OnComponentBeginOverlap` (`self.EnemyTrack`) (delegate `OnComponentBeginOverlap_Event_0`))
  (set `self.WallFollow` false)
  (`KismetSystemLibrary.Delay` 0.5)
  (set `self.WallFollow` true)
  (`GameplayStatics.PlaySound2D` "/Game/Audio/SFX/swoosh.swoosh" 1.0 1.0 0.0 null null)
  (add `PrimitiveComponent.OnComponentBeginOverlap` (`self.Collision`) (delegate `OnComponentBeginOverlap_Event_1`)))

(event `OnComponentBeginOverlap_Event_0`
  (params (OverlappedComponent :type "PrimitiveComponent Object Reference") (OtherActor :type "Actor Object Reference") (OtherComp :type "PrimitiveComponent Object Reference") (OtherBodyIndex :type Integer) (bFromSweep :type Boolean) (SweepResult :type "HitResult Structure (by ref)"))
  ;[1 1 1] Enemy Overlap Check
  (cast `/Game/Blueprints/Actors/BP_AICar` OtherActor)
  (`self.K2_SetActorRotation` (`KismetMathLibrary.FindLookAtRotation` (`self.K2_GetActorLocation`) (`self.K2_GetActorLocation`)))
  (set `self.WallFollow` false)
  (set `self.ToTrack` true))

(event `self.ReceiveDestroyed`
  ;[1 1 1] On Destroyed
  (set `self.ToTrack` false))

(fn `UserConstructionScript`)