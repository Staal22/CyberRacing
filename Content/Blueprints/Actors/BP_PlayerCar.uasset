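; Player car pawn that counts checkpoints and reloads or switches to the "Test" level once 15 are reached.
; On begin play it constrains movement to the plane spanned by its forward and right vectors and zeroes the camera's radial blur weight.
; An unconnected line-trace chain would smoothly roll the mesh to the ground normal, but it never runs.
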(event `self.Checkpoint`
  (bind _output_get (set `self.Checkpoints` (+ 1 (`self.Checkpoints`))))
  (if (>= _output_get 15)
    (`GameplayStatics.OpenLevel` "Test")
    (setmembers `PostProcessSettings` :`StructRef` (`CameraComponent.PostProcessSettings` (`self.Camera`)) :`WeightedBlendables` (make `WeightedBlendables` (`|MakeArray` (make `WeightedBlendable` 0.0 "/Game/Materials/PP_RadialBlur_1.PP_RadialBlur_1"))))))

(event `self.ReceiveBeginPlay`
  (`MovementComponent.SetPlaneConstraintEnabled` (`self.PawnMovementComponent`) true)
  (`MovementComponent.SetPlaneConstraintOrigin` (`self.PawnMovementComponent`) (`self.K2_GetActorLocation`))
  (`MovementComponent.SetPlaneConstraintFromVectors` (`self.PawnMovementComponent`) (`self.GetActorForwardVector`) (`self.GetActorRightVector`))
  (setmembers `PostProcessSettings` :`StructRef` (`CameraComponent.PostProcessSettings` (`self.Camera`)) :`WeightedBlendables` (make `WeightedBlendables` (`|MakeArray` (make `WeightedBlendable` 0.0 "/Game/Materials/PP_RadialBlur_1.PP_RadialBlur_1")))))

(event `self.ReceiveTick`
  (params (DeltaSeconds :type "Float (single-precision)")))

(fn `UserConstructionScript`)