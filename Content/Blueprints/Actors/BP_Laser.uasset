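; BP_Laser is a laser actor that redirects its Collision component when it overlaps something, apparently as a ricochet.
; BeginPlay binds the Collision begin-overlap event, which ignores the first player's pawn and the laser itself.
; Other overlaps keep roll and pitch but set world yaw to double the yaw derived from Collision's up vector and the sweep impact normal.
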(event `self.ReceiveBeginPlay`
  (add `PrimitiveComponent.OnComponentBeginOverlap` (`self.Collision`) (delegate `OnComponentBeginOverlap_Event_0`)))

(event `OnComponentBeginOverlap_Event_0`
  (params (OverlappedComponent :type "PrimitiveComponent Object Reference") (OtherActor :type "Actor Object Reference") (OtherComp :type "PrimitiveComponent Object Reference") (OtherBodyIndex :type Integer) (bFromSweep :type Boolean) (SweepResult :type "HitResult Structure (by ref)"))
  (if (== OtherActor (`GameplayStatics.GetPlayerPawn` 0))
    _
    (elif (not (== self OtherActor))
      (`SceneComponent.K2_SetWorldRotation` (`self.Collision`) (`KismetMathLibrary.MakeRotator` (.roll (`SceneComponent.K2_GetComponentRotation` (`self.Collision`))) (.pitch (`SceneComponent.K2_GetComponentRotation` (`self.Collision`))) (* (.yaw (`KismetMathLibrary.MakeRotFromZY` (`SceneComponent.GetUpVector` (`self.Collision`)) (`.ImpactNormal` (`GameplayStatics.BreakHitResult` SweepResult)))) 2.0)) false false))))

(fn `UserConstructionScript`)