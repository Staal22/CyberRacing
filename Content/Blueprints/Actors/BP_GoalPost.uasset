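; BP_GoalPost is the finish-line trigger that counts laps and decides wins and losses across the racing game's modes.
; GoalBox overlaps by AI cars advance the AI lap counter when AITrueLap is set, ending the game once LapMax is reached.
; Player overlaps show the win screen after enough Horde kills or final Race/Time Attack laps.
; Earlier laps require TrueLap, then clear it, increment the GameInstance counter and call the car's Lap.
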(event `self.GoalBox.OnComponentBeginOverlap`
  (params (OverlappedComponent :type "PrimitiveComponent Object Reference") (OtherActor :type "Actor Object Reference") (OtherComp :type "PrimitiveComponent Object Reference") (OtherBodyIndex :type Integer) (bFromSweep :type Boolean) (SweepResult :type "HitResult Structure (by ref)"))
  (bind _asbp_main_game_mode_base (cast `/Game/Blueprints/Gamemodes/BP_MainGameModeBase` (`GameplayStatics.GetGameMode`)))
  (bind _asracing_game_instance (cast `RacingGameInstance` (`GameplayStatics.GetGameInstance`)))
  ;[1 1 1] Lost to AI LULW
  (cast `/Game/Blueprints/Actors/BP_AICar` OtherActor
    (:`then`
      (if (`RacingGameInstance.bAITrueLap` _asracing_game_instance)
        (bind _asracing_game_instance_2 (cast `RacingGameInstance` (`GameplayStatics.GetGameInstance`)))
        (if (>= (`RacingGameInstance.AILapCounter` _asracing_game_instance_2) (`RacingGameInstance.LapMax` _asracing_game_instance_2))
          (`racing_gameGameModeBase.GameOver` _asbp_main_game_mode_base "Outraced by AI controlled car")
          (else
            (set `RacingGameInstance.AILapCounter` (+ (`RacingGameInstance.AILapCounter` _asracing_game_instance_2) 1) _asracing_game_instance_2)))))
    (:`CastFailed`
      (cast `/Game/Blueprints/Actors/BP_PlayerCar` OtherActor)
      (switch `string` (`RacingGameInstance.ActiveMode` _asracing_game_instance)
        (:`Horde`
          (if (>= (`racing_gameGameModeBase.KillCounter` _asbp_main_game_mode_base) 15)
            ;[1 1 1] Win
            (bind _returnvalue (`|CreateWidget` "/Game/Blueprints/Widgets/Widget_WinScreen.Widget_WinScreen_C" :!label _label))
            (`UserWidget.AddToViewport` _returnvalue 0)))
        (:`Race`
          (bind _btruelap (`RacingGameInstance.bTrueLap` _asracing_game_instance))
          (if _btruelap
            (bind _asracing_game_instance_3 (cast `RacingGameInstance` (`GameplayStatics.GetGameInstance`) :!label _label_2))
            (if (>= (`RacingGameInstance.LapCounter` _asracing_game_instance_3) (`RacingGameInstance.LapMax` _asracing_game_instance_3))
              (goto _label)
              (else
                (set `RacingGameInstance.bTrueLap` false _asracing_game_instance_3)
                (set `RacingGameInstance.LapCounter` (+ (`RacingGameInstance.LapCounter` _asracing_game_instance_3) 1) _asracing_game_instance_3)
                (bind _asbp_player_car (cast `/Game/Blueprints/Actors/BP_PlayerCar` (`GameplayStatics.GetPlayerPawn` 0)))
                (`PlayerCar.Lap` _asbp_player_car)))))
        (:`TimeAttack`
          (if _btruelap
            (goto _label_2)))))))

(fn `UserConstructionScript`)