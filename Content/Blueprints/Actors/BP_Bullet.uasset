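; BP_Bullet is a bullet actor that steers its mesh orientation to follow nearby ground and wall surfaces.
; Each tick a downward Visibility trace sets pitch from the ground normal, and a sideways trace, ignoring the player pawn, sets yaw from the wall normal.
; RInterpTo smooths the rotation while roll is preserved, and nothing changes without a ground hit.
; An opposite-side trace and yaw comparison are left unconnected.
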(event `self.ReceiveTick`
  (params (DeltaSeconds :type "Float (single-precision)"))
  (bind _returnvalue (`GameplayStatics.GetWorldDeltaSeconds`))
  (bind _bulletmesh (`self.BulletMesh`))
  (bind _bulletmesh_2 (`self.BulletMesh`))
  (bind _returnvalue_2 (`SceneComponent.K2_GetComponentLocation` _bulletmesh_2))
  (bind _returnvalue_3 (`SceneComponent.K2_GetComponentRotation` _bulletmesh))
  (bind _returnvalue_4 (`SceneComponent.K2_GetComponentLocation` (`self.BulletMesh`)))
  (bind _roll (.roll _returnvalue_3))
  (bind (_outhit _returnvalue_5) (`KismetSystemLibrary.LineTraceSingle` _returnvalue_4 (- _returnvalue_4 (`KismetMathLibrary.MakeVector` 0.0 0.0 (`self.TraceLengthZ`))) "TraceTypeQuery1"))
  (if _returnvalue_5
    (bind (_outhit_2 _returnvalue_6) (`KismetSystemLibrary.LineTraceSingle` _returnvalue_2 (- _returnvalue_2 (* (`SceneComponent.GetRightVector` _bulletmesh_2) (`self.TraceLengthY`))) "TraceTypeQuery1" false (`|MakeArray` (`GameplayStatics.GetPlayerPawn` 0) :!type "Actor Object Reference")))
    (if _returnvalue_6
      (bind _pitch (.pitch (`KismetMathLibrary.MakeRotFromYZ` (`SceneComponent.GetRightVector` _bulletmesh) (`.ImpactNormal` (`GameplayStatics.BreakHitResult` _outhit)))))
      (`SceneComponent.K2_SetWorldRotation` (`self.BulletMesh`) (`KismetMathLibrary.RInterpTo` _returnvalue_3 (`KismetMathLibrary.MakeRotator` _roll _pitch (.yaw (`KismetMathLibrary.MakeRotFromZY` (`SceneComponent.GetUpVector` _bulletmesh) (`.ImpactNormal` (`GameplayStatics.BreakHitResult` _outhit_2))))) _returnvalue 20.0) false false)
      (else
        (`SceneComponent.K2_SetWorldRotation` (`self.BulletMesh`) (`KismetMathLibrary.RInterpTo` _returnvalue_3 (`KismetMathLibrary.MakeRotator` _roll _pitch (.yaw _returnvalue_3)) _returnvalue 20.0) false false)))))

(fn `UserConstructionScript`)