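; Main game mode Blueprint that handles the game-over flow through a GameOver event taking a cause string.
; It creates the game-over widget, shows the cause as its death text and tints it by keyword match for damage, time or AI.
; After adding the widget to the viewport, it destroys every BP_Enemy actor and the player pawn.
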(event `self.GameOver`
  (params (Cause :type String))
  ;[1 1 1] Game Over
  (bind _returnvalue (`|CreateWidget` "/Game/Blueprints/Widgets/Widget_GameOverScreen.Widget_GameOverScreen_C"))
  (bind _causeofdeath (`/Game/Blueprints/Widgets/Widget_GameOverScreen.CauseOfDeath` _returnvalue))
  (`TextBlock.SetText` _causeofdeath (`KismetTextLibrary.Conv_StringToText` Cause))
  (if (`KismetStringLibrary.Contains` Cause "Damage")
    (`TextBlock.SetColorAndOpacity` _causeofdeath (make `SlateColor` (struct :`R` 0.869792 :`G` 0.027676 :`A` 1.0)))
    (elif (`KismetStringLibrary.Contains` Cause "Time")
      (`TextBlock.SetColorAndOpacity` _causeofdeath (make `SlateColor` (struct :`G` 0.031669 :`B` 1.0 :`A` 1.0)))
      (elif (`KismetStringLibrary.Contains` Cause "AI")
        (`TextBlock.SetColorAndOpacity` _causeofdeath (make `SlateColor` (struct :`R` 0.079982 :`G` 1.0 :`A` 1.0))))))
  (`UserWidget.AddToViewport` _returnvalue 0)
  (bind _outactors (`GameplayStatics.GetAllActorsOfClass` "/Game/Blueprints/Actors/BP_Enemy.BP_Enemy_C"))
  (for _array_element _outactors
    (`self.K2_DestroyActor` _array_element))
  (`self.K2_DestroyActor` (`GameplayStatics.GetPlayerPawn` 0)))

(fn `UserConstructionScript`)